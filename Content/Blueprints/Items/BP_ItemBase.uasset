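; Base item Blueprint that adds a pickup animation and self-removal to the parent class's Collected event.
; A DoOnce guard calls the parent logic, then a timeline drives the mesh's world scale from its mass scale multiplied by the SpinTrack curve.
; Alongside this, it speeds up the RotatingMovement roll and yaw spin, then destroys the actor after a short delay.
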(event `self.Collected`
  (bind _mesh (`self.Mesh`))
  (bind (_rotationrate_roll _rotationrate_pitch _rotationrate_yaw) (`KismetMathLibrary.BreakRotator` (`RotatingMovementComponent.RotationRate` (`self.RotatingMovement`))))
  (`/Engine/EditorBlueprintResources/StandardMacros.DoOnce` false
    (:`Completed`
      (`parent.Collected`)
      (`|ExecutionSequence`
        (:`then_0`
          (bind (_direction _spintrack) (`Timeline|Timeline`)
            (:`Update`
              (`SceneComponent.SetWorldScale3D` _mesh (`KismetMathLibrary.Conv_DoubleToVector` (* (`PrimitiveComponent.GetMassScale` _mesh "None") _spintrack))))))
        (:`then_1`
          (set `RotatingMovementComponent.RotationRate` (`KismetMathLibrary.MakeRotator` (* _rotationrate_roll 6.0) 0.0 (* _rotationrate_yaw 6.0)) (`self.RotatingMovement`))
          (`KismetSystemLibrary.Delay` 0.5)
          (`self.K2_DestroyActor`))))))

(fn `UserConstructionScript`)